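; Door Blueprint for a weight-balance mechanism that hands its logic to a C++ DoorBalance2 component.
; On BeginPlay it finds three trigger volume actors, passes their TriggerVolumeDoor2 zones to the component, then sets up its collision delegates and timeline.
; Helper functions add or subtract static mesh mass from BalanceMass and print it, but nothing here calls them, and SetTotalMassActor's summing loop is disconnected.
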(event `self.ReceiveBeginPlay`
  (bind _doorbalance2 (`self.DoorBalance2`))
  ;[1 1 1] C++ scripts
  ;;[1 1 1] on crée une référence vers BP_TriggerVolume + init méthodes de la classe DoorBalance
  (bind _returnvalue (`GameplayStatics.GetActorOfClass` "/Game/Ressources/Dynamique/BP/Features/triggers/BP_TriggerVolume_2_1.BP_TriggerVolume_2_1_C"))
  (bind _returnvalue_2 (`GameplayStatics.GetActorOfClass` "/Game/Ressources/Dynamique/BP/Features/triggers/BP_TriggerVolume_2_2.BP_TriggerVolume_2_2_C"))
  (bind _returnvalue_3 (`GameplayStatics.GetActorOfClass` "/Game/Ressources/Dynamique/BP/Features/triggers/BP_TriggerVolume_2_3.BP_TriggerVolume_2_3_C"))
  (`DoorBalance2.GetTriggersCollision` _doorbalance2 (`/Game/Ressources/Dynamique/BP/Features/triggers/BP_TriggerVolume_2_1.TriggerVolume_Door2` _returnvalue) (`/Game/Ressources/Dynamique/BP/Features/triggers/BP_TriggerVolume_2_2.TriggerVolume_Door2` _returnvalue_2) (`/Game/Ressources/Dynamique/BP/Features/triggers/BP_TriggerVolume_2_3.TriggerVolume_Door2` _returnvalue_3))
  (`DoorBalance2.SetupDelegateTriggerCollision` _doorbalance2)
  (`DoorBalance2.SetupTimeline` _doorbalance2))

(fn `addBalanceMass`
  (params (ActorAdded :type "Actor Object Reference"))
  (bind _returnvalue (`self.GetComponentByClass` ActorAdded "/Script/Engine.StaticMeshComponent"))
  (`/Engine/EditorBlueprintResources/StandardMacros.IsValid` _returnvalue
    (:`Is Valid`
      (bind _output_get (set `self.balanceMass` (+ (`PrimitiveComponent.GetMass` _returnvalue) (`self.balanceMass`))))
      (`KismetSystemLibrary.PrintString` (`KismetStringLibrary.Conv_DoubleToString` _output_get)))))

(fn `SetTotalMassActor`
  (params (Actors :type "Actor Object Reference")))

(fn `soustractBalanceMass`
  (params (ActorRemoved :type "Actor Object Reference"))
  (bind _returnvalue (`self.GetComponentByClass` ActorRemoved "/Script/Engine.StaticMeshComponent"))
  (`/Engine/EditorBlueprintResources/StandardMacros.IsValid` _returnvalue
    (:`Is Valid`
      (bind _output_get (set `self.balanceMass` (- (`self.balanceMass`) (`PrimitiveComponent.GetMass` _returnvalue))))
      (`KismetSystemLibrary.PrintString` (`KismetStringLibrary.Conv_DoubleToString` _output_get)))))

(fn `UserConstructionScript`)