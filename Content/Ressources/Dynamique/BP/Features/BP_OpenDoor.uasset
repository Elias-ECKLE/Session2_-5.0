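; BP_OpenDoor is a door actor tied to a weight trigger, with its logic delegated to the C++ DoorBalance component.
; On BeginPlay it finds BP_TriggerVolume, passes its TriggerVolumeDoor to DoorBalance, then has the component set up collision delegates and a timeline.
; The older Blueprint version, which sums overlapping mesh masses against MassMax to play or reverse a rotation timeline, remains disconnected.
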(event `triggerVolumeBeginCollision`
  (params (ActorCollided :type "Actor Object Reference"))
  ;[1 1 1] Blueprint script
  ;;[1 1 1] Collision
)

(event `self.DoorBalance.OnComponentActivated`
  (params (Component :type "ActorComponent Object Reference") (bReset :type Boolean))
  ;[1 1 1] C++ scripts
  ;;[1 1 1] On vérifie si le composant DoorBalance est bien présent
  (`KismetSystemLibrary.PrintString` "Script C++ DoorBalance readed"))

(event `triggerVolumeEndCollision`
  (params (ActorCollided :type "Actor Object Reference") (object :type "Object Object Reference"))
  ;[1 1 1] Blueprint script
  ;;[1 1 1] Collision
)

(event `self.ReceiveBeginPlay`
  (bind _doorbalance (`self.DoorBalance`))
  ;[1 1 1] C++ scripts
  ;;[1 1 1] on crée une référence vers BP_TriggerVolume + init méthodes de la classe DoorBalance
  (bind _returnvalue (`GameplayStatics.GetActorOfClass` "/Game/Ressources/Dynamique/BP/Features/triggers/BP_TriggerVolume.BP_TriggerVolume_C"))
  (bind _output_get (set `self.BP_TriggerVolume` _returnvalue))
  (`DoorBalance.GetTriggerCollision` _doorbalance (`/Game/Ressources/Dynamique/BP/Features/triggers/BP_TriggerVolume.TriggerVolume_Door` _output_get))
  (`DoorBalance.SetupDelegateTriggerCollision` _doorbalance)
  (`DoorBalance.SetupTimeline` _doorbalance))

(event `self.ReceiveTick`
  (params (DeltaSeconds :type "Float (single-precision)"))
  ;[1 1 1] Blueprint script
  ;;[1 1 1] Animation
)

(event `opensDoor`
  ;[1 1 1] Blueprint script
  ;;[1 1 1] Animation
)

(fn `addBalanceMass`
  (params (ActorAdded :type "Actor Object Reference"))
  (bind _returnvalue (`self.GetComponentByClass` ActorAdded "/Script/Engine.StaticMeshComponent"))
  (`/Engine/EditorBlueprintResources/StandardMacros.IsValid` _returnvalue
    (:`Is Valid`
      (bind _output_get (set `self.balanceMass` (+ (`PrimitiveComponent.GetMass` _returnvalue) (`self.balanceMass`))))
      (`KismetSystemLibrary.PrintString` (`KismetStringLibrary.Conv_DoubleToString` _output_get)))))

(fn `SetTotalMassActor`
  (params (Actors :type "Actor Object Reference")))

(fn `soustractBalanceMass`
  (params (ActorRemoved :type "Actor Object Reference"))
  (bind _returnvalue (`self.GetComponentByClass` ActorRemoved "/Script/Engine.StaticMeshComponent"))
  (`/Engine/EditorBlueprintResources/StandardMacros.IsValid` _returnvalue
    (:`Is Valid`
      (bind _output_get (set `self.balanceMass` (- (`self.balanceMass`) (`PrimitiveComponent.GetMass` _returnvalue))))
      (`KismetSystemLibrary.PrintString` (`KismetStringLibrary.Conv_DoubleToString` _output_get)))))

(fn `UserConstructionScript`)